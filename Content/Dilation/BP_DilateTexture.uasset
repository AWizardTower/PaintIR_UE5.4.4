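; BP_DilateTexture is a utility actor that generates a dilated texture in a render target.
; Its Dilate event triggers a scene capture, then draws M_Dilation into RT_Dilated.
; The construction script does nothing; disconnected nodes there would assign a static mesh and apply M_Unwarp to its material slots.
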(event `Dilate`
  (`SceneCaptureComponent2D.CaptureScene` (`self.SceneCaptureComponent2D`))
  (`KismetRenderingLibrary.DrawMaterialToRenderTarget` "/Game/Dilation/RT_Dilated.RT_Dilated" "/Game/Dilation/M_Dilation.M_Dilation"))

(fn `UserConstructionScript`)